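; Gameplay ability that toggles the player's weapon between equipped and unequipped, based on the Ability.Player.Equipped tag.
; Both branches play the same pistol equip montage while an Ability.BlockMontage tag is held.
; An Ability.Event.Equipped gameplay event times the swap: it calls EquipWeapon or UnEquipWeapon, links armed or unarmed anim layers and updates the tag.
; Only montage completion clears the block tag and ends the ability.
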(event `self.K2_ActivateAbility`
  (bind _returnvalue (`self.GetPlayerCharacterFromInfo`))
  (bind _returnvalue_2 (`self.GetPlayerCharacterFromInfo`))
  (`self.K2_CommitAbility`)
  (if (`GameplayTagAssetInterface.HasMatchingGameplayTag` (`self.GetOwnerAbilitySystemComponent`) (struct :`TagName` "Ability.Player.Equipped"))
    (`AbilitySystemBlueprintLibrary.AddGameplayTags` (`self.GetPlayerCharacterFromInfo`) (`BlueprintGameplayTagLibrary.MakeGameplayTagContainerFromTag` (`BlueprintGameplayTagLibrary.MakeLiteralGameplayTag` (struct :`TagName` "Ability.BlockMontage"))))
    (`AbilityTask_PlayMontageAndWait.CreatePlayMontageAndWaitProxy` "None" "/Game/Characters/Mannequins/Anims/Pistol/MM_Pistol_Equip_Montage.MM_Pistol_Equip_Montage"
      (:`then`
        (`AbilityTask_WaitGameplayEvent.WaitGameplayEvent` (struct :`TagName` "Ability.Event.Equipped") null
          (:`EventReceived`
            (bind _asbp_sigil_player (cast `/Game/Sigil/BPs/BP_SigilPlayer` _returnvalue))
            (`/Game/Sigil/BPs/BP_SigilPlayer.UnEquip_Weapon` _asbp_sigil_player)
            (`SkeletalMeshComponent.LinkAnimClassLayers` (`Character.Mesh` _returnvalue) "/Game/Sigil/Anim/ABP_PlayerLinkedLayers_UnArmed.ABP_PlayerLinkedLayers_UnArmed_C")
            (`AbilitySystemBlueprintLibrary.RemoveGameplayTags` (`self.GetPlayerCharacterFromInfo`) (`BlueprintGameplayTagLibrary.MakeGameplayTagContainerFromTag` (`BlueprintGameplayTagLibrary.MakeLiteralGameplayTag` (struct :`TagName` "Ability.Player.Equipped")))))))
      (:`OnCompleted`
        (`AbilitySystemBlueprintLibrary.RemoveGameplayTags` (`self.GetPlayerCharacterFromInfo`) (`BlueprintGameplayTagLibrary.MakeGameplayTagContainerFromTag` (`BlueprintGameplayTagLibrary.MakeLiteralGameplayTag` (struct :`TagName` "Ability.BlockMontage"))))
        (`self.K2_EndAbility`)))
    (else
      (`AbilitySystemBlueprintLibrary.AddGameplayTags` (`self.GetPlayerCharacterFromInfo`) (`BlueprintGameplayTagLibrary.MakeGameplayTagContainerFromTag` (`BlueprintGameplayTagLibrary.MakeLiteralGameplayTag` (struct :`TagName` "Ability.BlockMontage"))))
      (`AbilityTask_PlayMontageAndWait.CreatePlayMontageAndWaitProxy` "None" "/Game/Characters/Mannequins/Anims/Pistol/MM_Pistol_Equip_Montage.MM_Pistol_Equip_Montage"
        (:`then`
          (`AbilityTask_WaitGameplayEvent.WaitGameplayEvent` (struct :`TagName` "Ability.Event.Equipped") null
            (:`EventReceived`
              (bind _asbp_sigil_player_2 (cast `/Game/Sigil/BPs/BP_SigilPlayer` _returnvalue_2))
              (`/Game/Sigil/BPs/BP_SigilPlayer.Equip_Weapon` _asbp_sigil_player_2)
              (`SkeletalMeshComponent.LinkAnimClassLayers` (`Character.Mesh` _returnvalue_2) "/Game/Sigil/Anim/ABP_PlayerLinkedLayers_Armed.ABP_PlayerLinkedLayers_Armed_C")
              (`AbilitySystemBlueprintLibrary.AddGameplayTags` (`self.GetPlayerCharacterFromInfo`) (`BlueprintGameplayTagLibrary.MakeGameplayTagContainerFromTag` (`BlueprintGameplayTagLibrary.MakeLiteralGameplayTag` (struct :`TagName` "Ability.Player.Equipped")))))))
        (:`OnCompleted`
          (`AbilitySystemBlueprintLibrary.RemoveGameplayTags` (`self.GetPlayerCharacterFromInfo`) (`BlueprintGameplayTagLibrary.MakeGameplayTagContainerFromTag` (`BlueprintGameplayTagLibrary.MakeLiteralGameplayTag` (struct :`TagName` "Ability.BlockMontage"))))
          (`self.K2_EndAbility`))))))