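; Gameplay ability for the Sigil player's attack, which roots the character while an attack montage plays.
; It plays AM_Attacks from the section the player's AttackIndex selects in its StartSection array.
; A wait for the attack gameplay event starts alongside, but the player's Attack call runs immediately, not on event receipt.
; Only montage completion restores walk speed and ends the ability; interruption and cancellation are unhandled.
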(event `self.K2_ActivateAbility`
  (bind _returnvalue (`self.GetPlayerCharacterFromInfo`))
  (bind _returnvalue_2 (`self.GetPlayerCharacterFromInfo`))
  (bind _asbp_sigil_player (cast `/Game/Sigil/BPs/Player/BP_SigilPlayer` _returnvalue_2 :!pure true))
  (`self.K2_CommitAbility`)
  (set `CharacterMovementComponent.MaxWalkSpeed` 0.0 (`Character.CharacterMovement` _returnvalue_2))
  (`AbilityTask_PlayMontageAndWait.CreatePlayMontageAndWaitProxy` "None" "/Game/Sigil/Anim/AM/AM_Attacks.AM_Attacks" 1.0 (`|GetArrayItem` (`/Game/Sigil/BPs/Player/BP_SigilPlayer.Start Section` _asbp_sigil_player) (`/Game/Sigil/BPs/Player/BP_SigilPlayer.AttackIndex` _asbp_sigil_player))
    (:`then`
      (`AbilityTask_WaitGameplayEvent.WaitGameplayEvent` (struct :`TagName` "Ability.Event.Attack") null
        (:`then`
          (`/Game/Sigil/BPs/Player/BP_SigilPlayer.Attack` (cast `/Game/Sigil/BPs/Player/BP_SigilPlayer` _returnvalue :!pure true))
          (`KismetSystemLibrary.PrintString` "Next"))))
    (:`OnCompleted`
      (set `CharacterMovementComponent.MaxWalkSpeed` 500.0 (`Character.CharacterMovement` _returnvalue))
      (`self.K2_EndAbility`))))