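; GA_Sprint is a gameplay ability that toggles sprinting for the player character.
; On activation it checks the ability system component for the Ability.Sprint tag to choose a branch.
; It then adds or removes its GameplayTags variable on the character and switches CharacterMovement's MaxWalkSpeed between sprint and normal speed.
; The graph contains no EndAbility call.
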(event `self.K2_ActivateAbility`
  (if (`GameplayTagAssetInterface.HasMatchingGameplayTag` (`self.GetAbilitySystemComponentFromActorInfo`) (struct :`TagName` "Ability.Sprint"))
    (`AbilitySystemBlueprintLibrary.RemoveGameplayTags` (`self.GetPlayerCharacterFromInfo`) (`self.Gameplay Tags`))
    (set `CharacterMovementComponent.MaxWalkSpeed` 800.0 (`Character.CharacterMovement` (`self.GetPlayerCharacterFromInfo`)))
    (else
      (`AbilitySystemBlueprintLibrary.AddGameplayTags` (`self.GetPlayerCharacterFromInfo`) (`self.Gameplay Tags`))
      (set `CharacterMovementComponent.MaxWalkSpeed` 1200.0 (`Character.CharacterMovement` (`self.GetPlayerCharacterFromInfo`))))))