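; GA_Summon is a player gameplay ability that summons a BP_Spawn_Test actor where the camera is aiming.
; On activation it commits, then runs a long visibility line trace forward from the player character's follow camera.
; A hit spawns the actor at the impact point, and the ability ends immediately whether or not the trace hit.
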(event `self.K2_ActivateAbility`
  (bind _followcamera (`SigilPlayerCharacter.FollowCamera` (`self.GetPlayerCharacterFromInfo`)))
  (bind _returnvalue (`SceneComponent.K2_GetComponentLocation` _followcamera))
  (`self.K2_CommitAbility`)
  (bind (_outhit _returnvalue_2) (`KismetSystemLibrary.LineTraceSingle` _returnvalue (+ _returnvalue (* (`SceneComponent.GetForwardVector` _followcamera) 20000.0)) "TraceTypeQuery1"))
  (if _returnvalue_2
    (`|SpawnActorFromClass` "/Game/Sigil/BPs/Player/BP_Spawn_Test.BP_Spawn_Test_C" (`KismetMathLibrary.MakeTransform` (`.ImpactPoint` (`GameplayStatics.BreakHitResult` _outhit))) "Undefined" "MultiplyWithRoot" null null)
    (`self.K2_EndAbility`)
    (else
      (`self.K2_EndAbility`))))